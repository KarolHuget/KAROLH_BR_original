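; BP_BALL_01 is a player-controlled rolling ball driven by physics torque.
; Movement axis inputs apply acceleration-change torque to the sphere, scaled by a force multiplier.
; Any damage triggers a one-time camera fade, then reloads the current level.
; ChangeCameraView adjusts the spring arm's length and world pitch and yaw to reframe the camera.
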(event Game|Damage|EventAnyDamage
  (params (Damage :type Float%20%28single-precision%29) (DamageType :type Damage%20Type%20Object%20Reference) (InstigatedBy :type Controller%20Object%20Reference) (DamageCauser :type Actor%20Object%20Reference))
  (bind _returnvalue (Math|Float|MakeLiteralFloat 1.0))
  (|DoOnceMultiInput
    (:A%20Out
      (CameraFades|StartCameraFade :self (Game|GetPlayerCameraManager 0) :ToAlpha 1.0 :Duration _returnvalue)
      (Utilities|FlowControl|Delay _returnvalue)
      (bind _returnvalue_2 (Game|GetCurrentLevelName true))
      (Game|OpenLevel(byName) (Utilities|String|StringToName _returnvalue_2)))))

(event Input|AxisEvents|InputAxisForwardBack
  (params (AxisValue :type Float%20%28single-precision%29))
  ;[0 0.6562 0.4917] Ball Movement by torgue
  (Class|PrimitiveComponent|AddTorqueinRadians (Variables|Default|GetSphere) (Math|Vector|MakeVector (* AxisValue (Variables|Default|GetForceMultiply)) 0.0 0.0) "None" true))

(event Input|AxisEvents|InputAxisLeftRight
  (params (AxisValue :type Float%20%28single-precision%29))
  ;[0 0.6562 0.4917] Ball Movement by torgue
  (Class|PrimitiveComponent|AddTorqueinRadians (Variables|Default|GetSphere) (Math|Vector|MakeVector 0.0 (* AxisValue (Variables|Default|GetForceMultiply)) 0.0) "None" true))

(fn ConstructionScript)

(fn ChangeCameraView
  (params (Camera%20Position :type Float%20%28single-precision%29) (Camera%20Rotation%20Y :type Float%20%28single-precision%29) (Camera%20Rotation%20Z :type Float%20%28single-precision%29))
  (bind _springarm (Variables|Default|GetSpringArm))
  (Variables|/Script/Engine.SpringArmComponent|SetTargetArmLength _springarm Camera%20Position)
  (Transformation|SetWorldRotation _springarm (Math|Rotator|MakeRotator 0.0 Camera%20Rotation%20Y Camera%20Rotation%20Z) false false))